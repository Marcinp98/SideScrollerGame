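; Gameplay ability for a melee attack that damages live players around the avatar's combat socket.
; It plays a random montage from the avatar's attack list and waits for a montage-tag gameplay event.
; On the event, it damages players within a small sphere at that tag's socket, excluding itself, then ends.
; Random is re-evaluated per use, so montage and tag can mismatch; only the event path ends the ability.
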(event `self.K2_ActivateAbility`
  (bind _returnvalue (`self.GetAvatarActorFromActorInfo`))
  (bind _returnvalue_2 (message `CombatInterface.GetAttackMontages` (`self.GetAvatarActorFromActorInfo`)))
  (bind (_montage _montagetag) (break `TaggedMontage` (`KismetArrayLibrary.Array_Random` _returnvalue_2)))
  (`AbilityTask_PlayMontageAndWait.CreatePlayMontageAndWaitProxy` "None" _montage
    (:`then`
      (`AbilityTask_WaitGameplayEvent.WaitGameplayEvent` _montagetag null
        (:`EventReceived`
          (bind _returnvalue_3 (message `CombatInterface.GetCombatSocketLocation` _returnvalue _montagetag))
          (bind _outoverlappingactors (`MainAbilitySystemLibrary.GetLivePlayersWithinRadius` _returnvalue (`|MakeArray` _returnvalue) 45.0 _returnvalue_3))
          (for _array_element _outoverlappingactors
            (`self.CauseDamage` _array_element))
          (`self.K2_EndAbility`))))))