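; Enemy ranged attack gameplay ability that fires a projectile toward the avatar's combat target.
; On activation it plays a random tagged montage from the avatar's attack montages and waits for a gameplay event matching that montage's tag.
; The event spawns the projectile at the montage's socket tag, aimed at the target's location.
; The ability then ends without stopping the montage and prints a debug string.
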(event `self.K2_ActivateAbility`
  (bind _returnvalue (message `CombatInterface.GetAttackMontages` (`self.GetAvatarActorFromActorInfo`)))
  (bind _output_get (set `self.TaggedMontage` (`self.GetRandomTaggedMontageFromArray` _returnvalue)))
  (bind (_montage _montagetag _sockettag) (break `TaggedMontage` _output_get))
  (`AbilityTask_PlayMontageAndWait.CreatePlayMontageAndWaitProxy` "None" _montage 1.0 "None" false
    (:`then`
      (`AbilityTask_WaitGameplayEvent.WaitGameplayEvent` _montagetag null
        (:`EventReceived`
          ;[1 1 1] Rotacja Strzalu uwzględniająca pion
          (bind _returnvalue_2 (message `EnemyInterface.GetCombatTarget` (`self.GetAvatarActorFromActorInfo`)))
          (`/Engine/EditorBlueprintResources/StandardMacros.IsValid` _returnvalue_2
            (:`Is Valid`
              (set `self.TargetLocation` (`Actor.K2_GetActorLocation` _returnvalue_2)))
            (:`Is Not Valid`
              _))
          (`self.SpawnProjectile` (`self.TargetLocation`) _sockettag)
          (`self.K2_EndAbility`)
          (`KismetSystemLibrary.PrintString` (`KismetSystemLibrary.GetDisplayName` null)))))))